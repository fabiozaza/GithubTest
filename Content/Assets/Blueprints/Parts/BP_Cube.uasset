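; BP_Cube is a physics cube that can be picked up and dropped by a hand component.
; Pickup stores the hand and raises linear and angular damping; Drop clears it and lowers damping again.
; While held, Tick applies a spring-like force pulling the mesh toward a point in front of the hand, so it follows physically rather than being attached.
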(event `self.ReceiveTick`
  (params (DeltaSeconds :type "Float (single-precision)"))
  (bind _attachedobject (`self.attachedObject`))
  (`/Engine/EditorBlueprintResources/StandardMacros.IsValid` (`self.attachedObject`)
    (:`Is Valid`
      (`PrimitiveComponent.AddForce` (`self.StaticMesh`) (* (- (+ (`SceneComponent.K2_GetComponentLocation` _attachedobject) (* (`SceneComponent.GetForwardVector` _attachedobject) 300.0)) (`SceneComponent.K2_GetComponentLocation` (`self.StaticMesh`))) 5000.0) "None" false))))

(event `/Game/Assets/Interfaces/PickupInterface.Pickup`
  (params (Hand :type "SceneComponent Object Reference"))
  (set `self.attachedObject` Hand)
  (`PrimitiveComponent.SetLinearDamping` (`self.StaticMesh`) 20.0)
  (`PrimitiveComponent.SetAngularDamping` (`self.StaticMesh`) 20.0))

(event `/Game/Assets/Interfaces/PickupInterface.Drop`
  (params (Hand :type "SceneComponent Object Reference"))
  (set `self.attachedObject` null)
  (`PrimitiveComponent.SetLinearDamping` (`self.StaticMesh`) 0.01)
  (`PrimitiveComponent.SetAngularDamping` (`self.StaticMesh`) 0.0))

(fn `UserConstructionScript`)